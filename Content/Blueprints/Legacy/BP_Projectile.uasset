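; Legacy projectile that damages living FPSCharacters it overlaps, ignoring its own instigator apart from a debug message.
; On a valid hit it prints the target's name, spawns an explosion effect and sound at the target's location, then destroys itself.
; Damage comes from GE_Damage_Instant, applied to self through the target's Ability System Component.
; A timer set on BeginPlay destroys the projectile after a fixed lifetime.
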(event OnComponentBeginOverlap(Collision)
  (params (OverlappedComponent :type Primitive%20Component%20Object%20Reference) (OtherActor :type Actor%20Object%20Reference) (OtherComp :type Primitive%20Component%20Object%20Reference) (OtherBodyIndex :type Integer) (bFromSweep :type Boolean) (SweepResult :type Hit%20Result%20Structure%20%28by%20ref%29))
  (bind _returnvalue (Ability|GetAbilitySystemComponent OtherActor))
  (bind _returnvalue_2 (Transformation|GetActorLocation OtherActor))
  (Utilities|IsValid OtherActor
    (:Is%20Valid
      (bind _asfpscharacter (Utilities|Casting|CastToFPSCharacter OtherActor))
      (if (Variables|/Script/ProjectFPS.FPSCharacter|GetbIsAlive _asfpscharacter)
        (if (== (Game|GetInstigator) OtherActor)
          (Development|PrintString "Self-Damage")
          (else
            (Utilities|FlowControl|Sequence
              (:then_0
                (Development|PrintString (Utilities|GetDisplayName OtherActor)))
              (:then_1
                (Effects|SpawnEmitteratLocation "/Game/StarterContent/Particles/P_Explosion.P_Explosion" _returnvalue_2)
                (Audio|SpawnSoundatLocation "/Game/StarterContent/Audio/Explosion_Cue.Explosion_Cue" _returnvalue_2 "0, 0, 0" 1.0 1.0 0.0 0 0))
              (:then_2
                (Utilities|IsValid _returnvalue
                  (:Is%20Valid
                    (GameplayEffects|ApplyGameplayEffectToSelf :self _returnvalue :GameplayEffectClass "/Game/Blueprints/GameplayEffect/GE_Damage_Instant.GE_Damage_Instant_C" :Level 1.0))))
              (:then_3
                (Actor|DestroyActor)))))
        (else
          (Development|PrintString "이미 죽어있음!"))))))

(event EventBeginPlay
  (Utilities|Time|SetTimerbyFunctionName 0 "DestroyTimer" 7.0))

(fn ConstructionScript)

(fn DestroyTimer
  (Actor|DestroyActor))