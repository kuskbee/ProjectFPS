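; Gameplay ability meant to fire a BP_Projectile from the avatar pawn, though its spawn-and-end chain has no event triggering it, so it never runs.
; That chain spawns the projectile with the pawn as Instigator, then ends the ability.
; GetTransformFromAvatar places the spawn ahead of the avatar's eye point along control rotation.
; An unused GetTransformFromCamera offers a camera-based location with zero rotation.
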(fn GetTransformfromAvatar
  (bind _returnvalue (Ability|GetActorInfo))
  (bind (_owneractor _avataractor _playercontroller) (Utilities|Struct|BreakGameplayAbilityActorInfo _returnvalue))
  (bind _returnvalue_2 (Pawn|GetControlRotation _playercontroller :!class /Script/Engine.Controller))
  (return (Math|Transform|MakeTransform (+ (* (Math|Vector|GetForwardVector _returnvalue_2) 1e+02) (.OutLocation (Actor|GetActorEyesViewPoint _avataractor))) _returnvalue_2)))

(fn GetTransformfromCamera
  (bind _returnvalue (Game|GetPlayerCameraManager 0))
  (return (Math|Transform|MakeTransform (+ (Transformation|GetActorLocation _returnvalue) (* (Transformation|GetActorForwardVector _returnvalue) 5e+01)))))